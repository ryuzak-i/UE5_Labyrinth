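; BP_WidgetManager is a manager Blueprint that owns the player's UI: indicators, win and lose restart screens, the pause menu and interaction hints.
; BeginPlay adds the indicators, while events open restart or pause widgets, switching input mode, cursor and game pause, with pause toggles also notifying BP_AudioManager.
; Interaction hints toggle visibility and set text and icons by owner class, with doors checking BP_DataManager for the key.
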(event Custom|ShowWidgetWin
  ;[1 1 1] Widget Win
  (Development|PrintString "Show widget Win")
  (CallFunction|ShowWidgetRestart (Variables|Default|GetTitle_Text_Win) (Variables|Default|GetAction_Text_Restart)))

(event Custom|ShowWidgetLose
  ;[1 1 1] Widget Lose
  (Development|PrintString "Show widget Lose")
  (CallFunction|ShowWidgetRestart (Variables|Default|GetTitle_Text_Lose) (Variables|Default|GetAction_Text_Restart)))

(event Custom|HandleWidgetPause
  ;[1 1 1] Widget Pause
  (if (not (Game|IsGamePaused))
    (Development|PrintString "Show widget Pause")
    (CallFunction|ShowWidgetPause (Variables|Default|GetTitle_Text_Pause) (Variables|Default|GetAction_Text_Pause))
    (else
      (Development|PrintString "Hide widget Pause")
      (CallFunction|HideWidgetPause)))
  (bind _returnvalue (Actor|GetActorOfClass "/Game/Managers/BP_AudioManager.BP_AudioManager_C"))
  (Default|HandleMusicPause _returnvalue))

(event Custom|HandleWidgetInteractionHint
  (params (WidgetComponent :type Widget%20Component%20Object%20Reference))
  (bind _returnvalue (Rendering|IsVisible WidgetComponent))
  ;[1 1 1] Widget Interaction Hint
  (if (Utilities|IsValid WidgetComponent)
    (Rendering|SetVisibility WidgetComponent (not _returnvalue) false)
    (if _returnvalue
      (Development|PrintString "Show Interaction Hint")
      (else
        (Development|PrintString "Hide Interaction Hint")))
    (CallFunction|SetWidgetInteractionHint (UserInterface|GetWidget WidgetComponent) (Utilities|GetClass (Components|GetOwner WidgetComponent)))))

(event EventBeginPlay
  ;[1 1 1] Widget Player UI
  (bind _returnvalue (UserInterface|CreateWidget "/Game/Widgets/WBP_Indicators.WBP_Indicators_C" (Game|GetPlayerController 0)))
  (UserInterface|Viewport|AddtoViewport _returnvalue 0))

(fn ConstructionScript)

(fn ShowWidgetRestart
  (params (Title_Text :type Text) (Action_Text :type Text))
  (bind _returnvalue (Game|GetPlayerController 0))
  (bind _returnvalue_2 (UserInterface|CreateWidget "/Game/Widgets/Menu/WBP_Restart.WBP_Restart_C" _returnvalue Title_Text Action_Text))
  (UserInterface|Viewport|AddtoViewport _returnvalue_2 0)
  (Input|SetInputModeGameandUI _returnvalue _returnvalue_2 "DoNotLock" true true)
  (Game|SetGamePaused true)
  (Variables|/Script/Engine.PlayerController|SetbShowMouseCursor _returnvalue true)
  (Input|DisableInput (Game|GetPlayerCharacter 0) _returnvalue))

(fn ShowWidgetPause
  (params (TitleText :type Text) (ActionText :type Text))
  (bind _returnvalue (Game|GetPlayerController 0))
  (bind _returnvalue_2 (UserInterface|CreateWidget "/Game/Widgets/Menu/WBP_Pause.WBP_Pause_C" _returnvalue TitleText ActionText))
  (bind _output_get (Variables|Default|SetWidgetPause _returnvalue_2))
  (UserInterface|Viewport|AddtoViewport _output_get 0)
  (Input|SetInputModeGameandUI _returnvalue _output_get "DoNotLock" true false)
  (Game|SetGamePaused true)
  (Variables|/Script/Engine.PlayerController|SetbShowMouseCursor _returnvalue true))

(fn HideWidgetPause
  (bind _returnvalue (Game|GetPlayerController 0))
  (Widget|RemovefromParent (Variables|Default|GetWidgetPause))
  (Input|SetInputModeGameOnly _returnvalue false)
  (Game|SetGamePaused false)
  (Variables|/Script/Engine.PlayerController|SetbShowMouseCursor _returnvalue false))

(fn SetWidgetInteractionHint
  (params (Widget :type Object%20Object%20Reference) (Actor%20Class :type Actor%20Class%20Reference))
  (bind _aswbp_interaction_hint (Utilities|Casting|CastToWBP_InteractionHint Widget))
  (Variables|Default|SetWidgetInteractionHint _aswbp_interaction_hint)
  (if (== Actor%20Class "/Game/Interactables/BP_Door.BP_Door_C")
    (bind _returnvalue (Actor|GetActorOfClass "/Game/Managers/BP_DataManager.BP_DataManager_C"))
    (if (Variables|/Game/Managers/BP_DataManager.BP_DataManager_C|GetIsPlayerHaveKey _returnvalue)
      (Variables|/Game/Widgets/WBP_InteractionHint.WBP_InteractionHint_C|SetHint_Text (Variables|Default|GetWidgetInteractionHint) (Variables|Default|GetInteractionHint_UseKey))
      (Variables|/Game/Widgets/WBP_InteractionHint.WBP_InteractionHint_C|SetImage_KeyE_State (Variables|Default|GetWidgetInteractionHint) "Visible")
      (Variables|/Game/Widgets/WBP_InteractionHint.WBP_InteractionHint_C|SetImage_Block_State (Variables|Default|GetWidgetInteractionHint) "Collapsed")
      (else
        (Variables|/Game/Widgets/WBP_InteractionHint.WBP_InteractionHint_C|SetHint_Text (Variables|Default|GetWidgetInteractionHint) (Variables|Default|GetInteractionHint_FindKey))
        (Variables|/Game/Widgets/WBP_InteractionHint.WBP_InteractionHint_C|SetImage_Block_State (Variables|Default|GetWidgetInteractionHint) "Visible")
        (Variables|/Game/Widgets/WBP_InteractionHint.WBP_InteractionHint_C|SetImage_KeyE_State (Variables|Default|GetWidgetInteractionHint) "Collapsed")))
    (elif (== Actor%20Class "/Game/Interactables/BP_Key.BP_Key_C")
      (Variables|/Game/Widgets/WBP_InteractionHint.WBP_InteractionHint_C|SetHint_Text (Variables|Default|GetWidgetInteractionHint) (Variables|Default|GetInteractionHint_PickKey))
      (Variables|/Game/Widgets/WBP_InteractionHint.WBP_InteractionHint_C|SetImage_KeyE_State (Variables|Default|GetWidgetInteractionHint) "Visible")
      (elif (== Actor%20Class "/Game/Interactables/BP_Reward.BP_Reward_C")
        (Variables|/Game/Widgets/WBP_InteractionHint.WBP_InteractionHint_C|SetHint_Text (Variables|Default|GetWidgetInteractionHint) (Class|KismetTextLibrary|GetEmptyText))
        (Variables|/Game/Widgets/WBP_InteractionHint.WBP_InteractionHint_C|SetImage_KeyE_State (Variables|Default|GetWidgetInteractionHint) "Visible")))))