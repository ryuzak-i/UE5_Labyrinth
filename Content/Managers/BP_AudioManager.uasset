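; Central audio manager actor for game music, UI, key, door, win/lose and player footstep sounds.
; Music fades in at reduced pitch on BeginPlay, follows game pause through HandleMusicPause, and fades out on win or lose.
; A timeline, controlled by play/stop and rate functions, is meant to drive footsteps, which play at the player only when a downward sphere trace hits ground.
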(event Custom|KeyPick
  ;[1 1 1] Key & Door Sounds
  (Audio|PlaySound2D "/Game/Resources/Audio/SFX/key_pick.key_pick" (Variables|Default|GetKey_Volume) 1.0 0.0 0 0 false))

(event Custom|DoorOpen
  ;[1 1 1] Key & Door Sounds
  (Audio|PlaySound2D "/Game/Resources/Audio/SFX/door_open.door_open" (Variables|Default|GetDoor_Volume) 1.0 0.0 0 0 false))

(event Custom|PlaySoundWin
  ;[1 1 1] Handle Win & Lose Sounds
  (Audio|PlaySound2D "/Game/Resources/Audio/SFX/win.win" (Variables|Default|GetWin_Volume) 1.0 0.0 0 0)
  (Audio|Components|Audio|FadeOut (Variables|Default|GetMusic) 1.0 0.0 "Linear" :!class /Script/Engine.AudioComponent))

(event Custom|PlaySoundLose
  ;[1 1 1] Handle Win & Lose Sounds
  (Audio|PlaySound2D "/Game/Resources/Audio/SFX/lose.lose" (Variables|Default|GetLose_Volume) 1.0 0.0 0 0)
  (Audio|Components|Audio|FadeOut (Variables|Default|GetMusic) 1.0 0.0 "Linear" :!class /Script/Engine.AudioComponent))

(event Custom|PlayMusic
  ;[1 1 1] Music
  (bind _returnvalue (Audio|CreateSound2D "/Game/Resources/Audio/Music/music.music" 1.0 0.75 0.0 0))
  (bind _output_get (Variables|Default|SetMusic _returnvalue))
  (Audio|Components|Audio|FadeIn _output_get 1e+01 (Variables|Default|GetMusic_Volume) 0.0 "Linear" :!class /Script/Engine.AudioComponent))

(event Custom|UIButtonHover
  ;[1 1 1] UI Button Sound
  (Audio|PlaySound2D "/Game/Resources/Audio/SFX/button_over.button_over" (Variables|Default|GetUI_Button_Volume) 1.25 0.0 0 0))

(event EventBeginPlay
  (CallFunction|PlayMusic))

(fn ConstructionScript)

(fn TraceFootsteps
  (bind _returnvalue (Game|GetPlayerCharacter 0))
  (bind _returnvalue_2 (Transformation|GetActorLocation _returnvalue))
  (bind _capsulecomponent (Variables|/Script/Engine.Character|GetCapsuleComponent _returnvalue))
  (bind (_x _y _z) (Math|Vector|BreakVector _returnvalue_2))
  (bind _returnvalue_3 (Collision|SphereTraceByChannel _returnvalue_2 (Math|Vector|MakeVector _x _y (- _z (Components|Capsule|GetScaledCapsuleHalfHeight _capsulecomponent))) (Components|Capsule|GetScaledCapsuleRadius _capsulecomponent) "TraceTypeQuery1" false 0 "None"))
  (return _returnvalue_3))

(fn FootstepsPlay
  (bind _finished (CallFunction|TraceFootsteps))
  (if _finished
    (Audio|PlaySoundatLocation "/Game/Resources/Audio/SFX/Footsteps/SC_Footsteps.SC_Footsteps" (Transformation|GetActorLocation (Game|GetPlayerCharacter 0)) "0, 0, 0" 0.75 1.0 0.0 0 0 0 0)))

(fn SetFootstepsPlayRate
  (params (PlayRate :type Float%20%28double-precision%29))
  (Components|Timeline|SetPlayRate (Variables|Default|GetTL_Footsteps) PlayRate))

(fn HandleFootstepsPlay
  (params (IsPlay :type Boolean))
  (bind _tl_footsteps (Variables|Default|GetTL_Footsteps))
  (if IsPlay
    (Audio|Components|Audio|Play _tl_footsteps)
    (else
      (Audio|Components|Audio|Stop _tl_footsteps))))

(fn HandleMusicPause
  (bind _returnvalue (Game|IsGamePaused))
  (if _returnvalue
    _
    (else
      _))
  (Class|AudioComponent|SetPaused (Variables|Default|GetMusic) _returnvalue))