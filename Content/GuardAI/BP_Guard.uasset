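; Guard AI character that notifies the first-person player on capsule overlap and displays an eye widget for its sight state.
; It listens to AIC_Guard's eye-state changes and passes them to WBP_GuardSight.
; A proximity collision activates the widget, which toggles its visibility and rotates toward the player camera each tick while active.
; SetMovementSpeed maps idle, walk and chase modes to max walk speed.
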(event OnComponentBeginOverlap(CapsuleComponent)
  (params (OverlappedComponent :type Primitive%20Component%20Object%20Reference) (OtherActor :type Actor%20Object%20Reference) (OtherComp :type Primitive%20Component%20Object%20Reference) (OtherBodyIndex :type Integer) (bFromSweep :type Boolean) (SweepResult :type Hit%20Result%20Structure%20%28by%20ref%29))
  (bind _returnvalue (Game|GetPlayerCharacter 0))
  ;[1 1 1] Guard overlap Player
  (if (== OtherActor _returnvalue)
    (Development|PrintString "Guard overlap Player" true true "(R=0.000000,G=0.660000,B=1.000000,A=1.000000)" 1e+01)
    (bind _asbp_first_person_character (Utilities|Casting|CastToBP_FirstPersonCharacter _returnvalue))
    (Default|OverlapEnemy _asbp_first_person_character)))

(event OnComponentBeginOverlap(EyeWidgetCollision)
  (params (OverlappedComponent :type Primitive%20Component%20Object%20Reference) (OtherActor :type Actor%20Object%20Reference) (OtherComp :type Primitive%20Component%20Object%20Reference) (OtherBodyIndex :type Integer) (bFromSweep :type Boolean) (SweepResult :type Hit%20Result%20Structure%20%28by%20ref%29))
  ;[1 1 1] Handle Activating and Deactivating Eye Widget
  (if (== OtherActor (Game|GetPlayerCharacter 0))
    (Components|Activation|Activate (Variables|Default|GetEyeWidget) false)))

(event OnComponentEndOverlap(EyeWidgetCollision)
  (params (OverlappedComponent :type Primitive%20Component%20Object%20Reference) (OtherActor :type Actor%20Object%20Reference) (OtherComp :type Primitive%20Component%20Object%20Reference) (OtherBodyIndex :type Integer))
  ;[1 1 1] Handle Activating and Deactivating Eye Widget
  (if (== OtherActor (Game|GetPlayerCharacter 0))
    (Components|Activation|Deactivate (Variables|Default|GetEyeWidget))))

(event OnComponentActivated(EyeWidget)
  (params (Component :type Actor%20Component%20Object%20Reference) (bReset :type Boolean))
  ;[1 1 1] Handle Eye Widget visibility
  (Development|PrintString "Guard eye Activated")
  (Rendering|SetVisibility (Variables|Default|GetEyeWidget) true false))

(event OnComponentDeactivated(EyeWidget)
  (params (Component :type Actor%20Component%20Object%20Reference))
  ;[1 1 1] Handle Eye Widget visibility
  (Development|PrintString "Guard eye Deactivated")
  (Rendering|SetVisibility (Variables|Default|GetEyeWidget) false false))

(event Custom|RotateEyeWidget
  (bind _eyewidget (Variables|Default|GetEyeWidget))
  ;[1 1 1] Rotate Eye Widget
  (Transformation|SetWorldRotation _eyewidget (Math|Rotator|FindLookatRotation (Transformation|GetWorldLocation _eyewidget) (Transformation|GetWorldLocation (Variables|/Script/Engine.PlayerCameraManager|GetTransformComponent (Game|GetPlayerCameraManager 0)))) false false))

(event Custom|OnChangeEyeState_Event
  (params (EyeState :type E_GuardStates%20Enum :default "NewEnumerator0"))
  ;[1 1 1] Observer to change Eye Widget state
  (bind _aswbp_guard_sight (Utilities|Casting|CastToWBP_GuardSight (UserInterface|GetWidget (Variables|Default|GetEyeWidget))))
  (Default|SetEyeState _aswbp_guard_sight EyeState))

(event EventBeginPlay
  ;[1 1 1] Observer to change Eye Widget state
  (bind _asaic_guard (Utilities|Casting|CastToAIC_Guard (AI|GetAIController self)))
  (EventDispatchers|BindEventtoOnChangeEyeState _asaic_guard (delegate Custom|OnChangeEyeState_Event)))

(event EventTick
  (params (DeltaSeconds :type Float%20%28single-precision%29))
  ;[1 1 1] Handle Eye Widget Rotating
  (if (Components|Activation|IsActive (Variables|Default|GetEyeWidget))
    (CallFunction|RotateEyeWidget)))

(fn ConstructionScript)

(fn SetMovementSpeed
  (params (Speed :type E_GuardMovementSpeed%20Enum :default "NewEnumerator0"))
  (Variables|/Script/Engine.CharacterMovementComponent|SetMaxWalkSpeed (Variables|Character|GetCharacterMovement) (Utilities|Select :Index Speed :NewEnumerator0 (Variables|Default|GetIdleSpeed) :NewEnumerator1 (Variables|Default|GetWalkSpeed) :NewEnumerator2 (Variables|Default|GetChaseSpeed)))
  (return))