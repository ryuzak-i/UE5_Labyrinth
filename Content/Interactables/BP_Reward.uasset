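; BP_Reward is an interactable pickup with a spinning cube that the player collects by pressing E.
; A Timeline rotates the cube, while player overlap enables or disables actor input and passes the hint Widget to BP_WidgetManager on both enter and exit.
; On E, it destroys the widget and itself, then calls PickReward on the BP_FirstPersonCharacter cached at overlap.
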(event EventBeginPlay
  ;[1 1 1] Cube Rotation
  (bind _rotation (Timeline|Timeline Play)
    (:Update
      (Transformation|SetRelativeRotation (Variables|Default|GetCube) (Math|Rotator|MakeRotator (* _rotation 3.6e+02) (* _rotation 3.6e+02) (* _rotation 3.6e+02)) false false))))

(event Collision|EventActorBeginOverlap
  (params (OtherActor :type Actor%20Object%20Reference))
  (bind _returnvalue (Game|GetPlayerCharacter 0))
  (if (== OtherActor _returnvalue)
    (bind _asbp_first_person_character (Utilities|Casting|CastToBP_FirstPersonCharacter _returnvalue))
    (Development|PrintString "Player overlap Reward")
    (Input|EnableInput (Game|GetPlayerController 0))
    (bind _returnvalue_2 (Actor|GetActorOfClass "/Game/Managers/BP_WidgetManager.BP_WidgetManager_C"))
    (Default|HandleWidgetInteractionHint _returnvalue_2 (Variables|Default|GetWidget))))

(event Collision|EventActorEndOverlap
  (params (OtherActor :type Actor%20Object%20Reference))
  (if (== OtherActor (Game|GetPlayerCharacter 0))
    (Input|DisableInput (Game|GetPlayerController 0))
    (bind _returnvalue (Actor|GetActorOfClass "/Game/Managers/BP_WidgetManager.BP_WidgetManager_C"))
    (Default|HandleWidgetInteractionHint _returnvalue (Variables|Default|GetWidget))))

(event Input|KeyboardEvents|E
  (params (Key :type Key%20Structure :default "None"))
  (:Pressed
    (Development|PrintString "Player pick Reward")
    (Utilities|FlowControl|Sequence
      (:then_0
        (Components|DestroyComponent (Variables|Default|GetWidget)))
      (:then_1
        (Actor|DestroyActor))
      (:then_2
        (Default|PickReward (stale Collision|EventActorBeginOverlap _asbp_first_person_character))))))

(fn ConstructionScript)