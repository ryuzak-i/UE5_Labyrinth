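; BP_Door is an interactable door that the player unlocks with a key and that then sinks away.
; Player overlap enables or disables its input and passes its widget to BP_WidgetManager to handle the interaction hint.
; Pressing E checks and clears the key flag in BP_DataManager, removes the widget and triggers BP_AudioManager's door sound.
; A Timeline lowers the Cube, then destroys the actor.
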(event EventBeginPlay
  ;[1 1 1] Save Managers
  (Utilities|FlowControl|Sequence
    (:then_0
      (bind _returnvalue (Actor|GetActorOfClass "/Game/Managers/BP_DataManager.BP_DataManager_C"))
      (Variables|Default|SetDataManager _returnvalue))
    (:then_1
      (bind _returnvalue_2 (Actor|GetActorOfClass "/Game/Managers/BP_WidgetManager.BP_WidgetManager_C"))
      (Variables|Default|SetWidgetManager _returnvalue_2))))

(event Collision|EventActorBeginOverlap
  (params (OtherActor :type Actor%20Object%20Reference))
  (bind _returnvalue (Game|GetPlayerCharacter 0))
  (if (== OtherActor _returnvalue)
    (Utilities|Casting|CastToBP_FirstPersonCharacter _returnvalue)
    (Development|PrintString "Player overlap Door")
    (Input|EnableInput (Game|GetPlayerController 0))
    (Default|HandleWidgetInteractionHint (Variables|Default|GetWidgetManager) (Variables|Default|GetWidget))))

(event Collision|EventActorEndOverlap
  (params (OtherActor :type Actor%20Object%20Reference))
  (if (== OtherActor (Game|GetPlayerCharacter 0))
    (Input|DisableInput (Game|GetPlayerController 0))
    (Default|HandleWidgetInteractionHint (Variables|Default|GetWidgetManager) (Variables|Default|GetWidget))))

(event Input|KeyboardEvents|E
  (params (Key :type Key%20Structure :default "None"))
  (:Pressed
    (if (Variables|/Game/Managers/BP_DataManager.BP_DataManager_C|GetIsPlayerHaveKey (Variables|Default|GetDataManager))
      (Utilities|FlowControl|Sequence
        (:then_0
          (Components|DestroyComponent (Variables|Default|GetWidget)))
        (:then_1
          (Variables|/Game/Managers/BP_DataManager.BP_DataManager_C|SetIsPlayerHaveKey (Variables|Default|GetDataManager) false))
        (:then_2
          (bind _returnvalue (Actor|GetActorOfClass "/Game/Managers/BP_AudioManager.BP_AudioManager_C"))
          (Default|DoorOpen _returnvalue))
        (:then_3
          (Development|PrintString "Door open")
          (bind _disappear (Timeline|Timeline Play)
            (:Update
              (Transformation|SetRelativeLocation (Variables|Default|GetCube) (Math|Vector|MakeVector 0.0 0.0 (* _disappear -5e+02)) false false))
            (:Finished
              (Development|PrintString "Door destroy")
              (Actor|DestroyActor))))))))

(fn ConstructionScript)