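; BP_Key is a pickup key that the player collects by pressing E while overlapping it.
; Overlap begin and end enable or disable the actor's input and pass its Widget to BP_WidgetManager's interaction hint handler.
; On pickup it destroys the widget and itself, triggers BP_AudioManager's KeyPick, then increments KeysCount and sets IsPlayerHaveKey on BP_DataManager.
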(event EventBeginPlay
  ;[1 1 1] Save Managers
  (Utilities|FlowControl|Sequence
    (:then_0
      (bind _returnvalue (Actor|GetActorOfClass "/Game/Managers/BP_DataManager.BP_DataManager_C"))
      (Variables|Default|SetDataManager _returnvalue))
    (:then_1
      (bind _returnvalue_2 (Actor|GetActorOfClass "/Game/Managers/BP_WidgetManager.BP_WidgetManager_C"))
      (Variables|Default|SetWidgetManager _returnvalue_2))))

(event Collision|EventActorBeginOverlap
  (params (OtherActor :type Actor%20Object%20Reference))
  (bind _returnvalue (Game|GetPlayerCharacter 0))
  (if (== OtherActor _returnvalue)
    (Utilities|Casting|CastToBP_FirstPersonCharacter _returnvalue)
    (Development|PrintString "Player overlap Key")
    (Input|EnableInput (Game|GetPlayerController 0))
    (Default|HandleWidgetInteractionHint (Variables|Default|GetWidgetManager) (Variables|Default|GetWidget))))

(event Collision|EventActorEndOverlap
  (params (OtherActor :type Actor%20Object%20Reference))
  (if (== OtherActor (Game|GetPlayerCharacter 0))
    (Input|DisableInput (Game|GetPlayerController 0))
    (Default|HandleWidgetInteractionHint (Variables|Default|GetWidgetManager) (Variables|Default|GetWidget))))

(event Input|KeyboardEvents|E
  (params (Key :type Key%20Structure :default "None"))
  (:Pressed
    (Development|PrintString "Key pick")
    (Utilities|FlowControl|Sequence
      (:then_0
        (Components|DestroyComponent (Variables|Default|GetWidget)))
      (:then_1
        (Actor|DestroyActor))
      (:then_2
        (bind _returnvalue (Actor|GetActorOfClass "/Game/Managers/BP_AudioManager.BP_AudioManager_C"))
        (Default|KeyPick _returnvalue))
      (:then_3
        (bind _returnvalue_2 (Actor|GetActorOfClass "/Game/Managers/BP_DataManager.BP_DataManager_C"))
        (Variables|/Game/Managers/BP_DataManager.BP_DataManager_C|SetKeysCount _returnvalue_2 (+ (Variables|/Game/Managers/BP_DataManager.BP_DataManager_C|GetKeysCount _returnvalue_2) 1))
        (Variables|/Game/Managers/BP_DataManager.BP_DataManager_C|SetIsPlayerHaveKey _returnvalue_2 true)))))

(fn ConstructionScript)